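; Anim notify for weapon fire that plays a gunshot sound and spawns a rifle muzzle flash on an ALS character.
; When the mesh is visible, it spawns the sound attached to the mesh and sets its FireSoundType integer parameter from the notify's setting.
; If that sound is valid and the pawn owner is an ALS_BaseCharacter, it spawns the particle at the weapon's muzzle socket, scaled to a tenth.
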(fn `Received_Notify`
  (params (MeshComp :type "SkeletalMeshComponent Object Reference") (Animation :type "AnimSequenceBase Object Reference"))
  (returns (ReturnValue :type Boolean))
  (if (`SceneComponent.IsVisible` MeshComp)
    ;[1 1 1] 声音
    (bind _returnvalue (`GameplayStatics.SpawnSoundAttached` (`self.Sound`) MeshComp (`self.AttachPointName`) (0.0 0.0 0.0) (struct) "KeepRelativeOffset" false (`self.VolumeMultiplier`) (`self.PitchMultiplier`) 0.0 null null))
    (`/Engine/EditorBlueprintResources/StandardMacros.IsValid` _returnvalue
      (:`Is Valid`
        (`AudioComponent.SetIntParameter` _returnvalue "FireSoundType" (`KismetMathLibrary.Conv_ByteToInt` (`self.FireSoundType`)))
        (bind _asals_base_character (cast `/Game/Blueprints/ALS_BaseCharacter` (`AnimInstance.TryGetPawnOwner` (`SkeletalMeshComponent.GetAnimInstance` MeshComp))))
        (bind (_returnvalue_location _returnvalue_rotation _returnvalue_scale) (`KismetMathLibrary.BreakTransform` (`SceneComponent.GetSocketTransform` (`/Game/Blueprints/Item/Weapon/JN_Item_Weapon_Base.SkeletalMeshWeapon` (`/Game/Blueprints/ALS_BaseCharacter.Weapon` _asals_base_character)) "b_gun_muzzleflashSocket" "RTS_World")))
        (`GameplayStatics.SpawnEmitterAtLocation` "/Game/InfinityBladeEffects/Effects/FX_Monsters/FX_Monster_Chicken/P_Rifle_Fire.P_Rifle_Fire" _returnvalue_location _returnvalue_rotation (* _returnvalue_scale 0.1))
        (return false)))))