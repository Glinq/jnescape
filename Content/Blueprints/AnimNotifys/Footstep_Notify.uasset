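; Footstep_Notify is an animation notify that plays footstep sounds on a mesh when the notify fires during an animation.
; If the mesh is visible, it spawns the configured sound attached at a named point with adjustable volume and pitch.
; It then passes the notify's footstep type to the spawned audio component as the integer "FootstepType" parameter, letting the sound vary by step type.
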(fn `Received_Notify`
  (params (MeshComp :type "SkeletalMeshComponent Object Reference") (Animation :type "AnimSequenceBase Object Reference"))
  (returns (ReturnValue :type Boolean))
  (if (`SceneComponent.IsVisible` MeshComp)
    (bind _returnvalue (`GameplayStatics.SpawnSoundAttached` (`self.Sound`) MeshComp (`self.AttachPointName`) (0.0 0.0 0.0) (struct) "KeepRelativeOffset" false (`self.VolumeMultiplier`) (`self.PitchMultiplier`) 0.0 null null))
    (`/Engine/EditorBlueprintResources/StandardMacros.IsValid` _returnvalue
      (:`Is Valid`
        (`AudioComponent.SetIntParameter` _returnvalue "FootstepType" (`KismetMathLibrary.Conv_ByteToInt` (`self.FootstepType`)))
        (return false)))))